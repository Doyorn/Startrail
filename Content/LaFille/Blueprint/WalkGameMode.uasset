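; Game mode for a walking level that builds the initial strip of floor and scenery when play begins.
; BeginPlay spawns a fixed run of BP_FloorTiles, then a run of BP_Fond background pieces.
; Each spawned piece supplies its attach transform, stored as the next spawn point for its type, so pieces chain end to end along two independent tracks.
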(event EventBeginPlay
  (Utilities|FlowControl|Sequence
    (:then_0
      ;[1 1 1] Le nombre de sol a ajouté
      (for _index (range 0 2)
        (CallFunction|AddFloorTiles)))
    (:then_1
      (for _index_2 (range 0 3)
        (CallFunction|AddBackground)))))

(fn ConstructionScript)

(fn AddFloorTiles
  (bind _returnvalue (Game|SpawnActorfromClass "/Game/ObjetsPhysique/LeSolInfini/FloorInfinie/BP_FloorTiles.BP_FloorTiles_C" (Variables|Default|GetNextSpawnPointFloor) "Undefined" 0 0))
  (bind _asbp_floor_tiles (Utilities|Casting|CastToBP_FloorTiles _returnvalue))
  (bind _attachtransformtiles (Default|GetAttachTransform _asbp_floor_tiles))
  (Variables|Default|SetNextSpawnPointFloor _attachtransformtiles))

(fn AddBackground
  (bind _returnvalue (Game|SpawnActorfromClass "/Game/ObjetsPhysique/Fond/BP_Fond.BP_Fond_C" (Variables|Default|GetNextSpawnPointBF) "Undefined" 0 0))
  (bind _asbp_fond (Utilities|Casting|CastToBP_Fond _returnvalue))
  (bind _attachtransformfond (Default|GetAttachTransform _asbp_fond))
  (Variables|Default|SetNextSpawnPointBF _attachtransformfond))