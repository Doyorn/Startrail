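; Infinite-floor tile that decorates itself with random 2D sprites, apparently plants, when it spawns.
; BeginPlay chains duplicated loop macros and DoOnce nodes to add Paper sprites with random counts, positions and scales in several depth bands, plus an occasional extra sprite.
; When LaFille overlaps BoxEndTrigger, the tile calls AddFloorTiles on WalkGameMode and destroys itself.
; GetAttachTransform exposes the AttachPoint world transform.
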(event OnComponentBeginOverlap(BoxEndTrigger)
  (params (OverlappedComponent :type Primitive%20Component%20Object%20Reference) (OtherActor :type Actor%20Object%20Reference) (OtherComp :type Primitive%20Component%20Object%20Reference) (OtherBodyIndex :type Integer) (bFromSweep :type Boolean) (SweepResult :type Hit%20Result%20Structure%20%28by%20ref%29))
  (Utilities|Casting|CastToLaFille OtherActor)
  (bind _aswalk_game_mode (Utilities|Casting|CastToWalkGameMode (Game|GetGameMode)))
  (Default|AddFloorTiles _aswalk_game_mode)
  (Actor|DestroyActor))

(event Collision|EventActorBeginOverlap
  (params (OtherActor :type Actor%20Object%20Reference)))

(event EventTick
  (params (DeltaSeconds :type Float%20%28single-precision%29)))

(event EventBeginPlay
  (bind _returnvalue (Math|Random|RandomFloatinRange 0.127927 0.129927))
  (bind _returnvalue_2 (Math|Random|RandomFloatinRange 0.127927 0.129927))
  (bind _returnvalue_3 (Math|Random|RandomFloatinRange 0.1 0.2))
  (bind _returnvalue_4 (Math|Random|RandomFloatinRange 0.15 0.2))
  (bind _returnvalue_5 (Math|Random|RandomFloatinRange 0.15 0.2))
  ;[1 1 1] Herbe 1
  ;;[1 1 1] Quand le sol se créer
  (|Forloopmaisenmieux (Math|Random|RandomIntegerinRange 0 5)
    (:C'est%200
      (Development|PrintString "Ah c un 0"))
    (:Ya%20des%20plantes%20ok
      (AddComponent|AddPaperSpriteComponent false (Math|Transform|MakeTransform (Math|Vector|MakeVector (Math|Random|RandomFloatinRange 0.0 1.2e+03) (Math|Random|RandomFloatinRange -89.0 -91.0) 3e+01) "0, 0, 0" (Math|Vector|MakeVector _returnvalue _returnvalue _returnvalue)))))
  (Utilities|FlowControl|DoOnce false
    (:Completed
      (|Forloopmaisenmieux_2 (Math|Random|RandomIntegerinRange 0 10)
        (:C'est%200
          (Development|PrintString "Ah c un 0"))
        (:Ya%20des%20plantes%20ok
          (AddComponent|AddPaperSpriteComponent false (Math|Transform|MakeTransform (Math|Vector|MakeVector (Math|Random|RandomFloatinRange 0.0 1.2e+03) (Math|Random|RandomFloatinRange -89.0 -91.0) 4e+01) "0, 0, 0" (Math|Vector|MakeVector _returnvalue_2 _returnvalue_2 _returnvalue_2)))))
      (Utilities|FlowControl|DoOnce false
        (:Completed
          (|Forloopmaisenmieux_2_2 (Math|Random|RandomIntegerinRange 0 50)
            (:C'est%200
              (Development|PrintString "Ah c un 0"))
            (:Ya%20des%20plantes%20ok
              (AddComponent|AddPaperSpriteComponent false (Math|Transform|MakeTransform (Math|Vector|MakeVector (Math|Random|RandomFloatinRange 0.0 1.2e+03) (Math|Random|RandomFloatinRange -2e+02 -2.1e+02) 0.0) "0, 0, 0" (Math|Vector|MakeVector _returnvalue_3 _returnvalue_3 _returnvalue_3)))))
          (Utilities|FlowControl|DoOnce false
            (:Completed
              (|Forloopmaisenmieux_2_2_2 (Math|Random|RandomIntegerinRange 0 4)
                (:C'est%200
                  _)
                (:Ya%20des%20plantes%20ok
                  (AddComponent|AddPaperSpriteComponent false (Math|Transform|MakeTransform (Math|Vector|MakeVector (Math|Random|RandomFloatinRange 0.0 1.2e+03) (Math|Random|RandomFloatinRange -2.1e+02 -2.2e+02) 0.0) "0, 0, 0" (Math|Vector|MakeVector _returnvalue_4 _returnvalue_4 _returnvalue_4)))))
              (Utilities|FlowControl|DoOnce false
                (:Completed
                  (|Forloopmaisenmieux_2_2_2_2 (Math|Random|RandomIntegerinRange 10 20)
                    (:C'est%200
                      _)
                    (:Ya%20des%20plantes%20ok
                      (AddComponent|AddPaperSpriteComponent false (Math|Transform|MakeTransform (Math|Vector|MakeVector (Math|Random|RandomFloatinRange 0.0 1.2e+03) (Math|Random|RandomFloatinRange 95.0 1e+02) 0.0) "0, 0, 0" (Math|Vector|MakeVector _returnvalue_5 _returnvalue_5 _returnvalue_5)))))
                  (Utilities|FlowControl|DoOnce false
                    (:Completed
                      (if (< (Math|Random|RandomIntegerinRange 5 100) 10)
                        (AddComponent|AddPaperSpriteComponent false (Math|Transform|MakeTransform (Math|Vector|MakeVector (Math|Random|RandomFloatinRange 0.0 1.5e+03) (Math|Random|RandomFloatinRange 3e+01 3e+01) (Math|Random|RandomFloatinRange 2e+01 3e+01)) "0, 0, 0" (Math|Vector|MakeVector 0.15 0.0 0.15)))))))))))))))

(fn ConstructionScript)

(fn GetAttachTransform
  (return (Transformation|GetWorldTransform (Variables|Default|GetAttachPoint))))